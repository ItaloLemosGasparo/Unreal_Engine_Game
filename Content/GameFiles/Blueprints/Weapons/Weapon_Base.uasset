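; Base weapon Blueprint for the player's guns, built around an EBBarrel ballistics component that handles firing and ammo.
; Before each shot, a camera line trace finds the target and rotates the barrel along a calculated ballistic aim direction, resetting it when nothing is hit.
; Each shot increases barrel spread, updates crosshair spread, adds random camera recoil and plays the fire animation.
; Reloading plays its animation and sets the barrel's ammo from weapon capacity.
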(event ShotFired(EBBarrel)
  ;[1 0 0] Do Every Shoot
  (Utilities|FlowControl|Sequence
    (:then_0
      (CallFunction|Weapon/BarrelSpreadandRecoil))
    (:then_1
      (Components|Animation|PlayAnimation (Variables|Components|GetWeaponMesh) (Variables|WeaponCaracteristics|GetFireAnimation self) false))))

(event BeforeShotFired(EBBarrel)
  ;[1 0 0] Before Shoot
  (CallFunction|AimCorrection))

(event Custom|AimCorrection
  (bind _returnvalue (Game|GetPlayerCameraManager 0))
  (bind _ebbarrel (Variables|Components|GetEBBarrel))
  (bind _returnvalue_2 (Camera|GetCameraLocation _returnvalue))
  ;[1 0 0] Get target location and adjust EBBARREL rotation to hit the target.
  (bind _outactors (Actor|GetAllActorsOfClass "/Game/AdvancedLocomotionV4/Blueprints/CharacterLogic/PlayerCharacter.PlayerCharacter_C"))
  (bind _outhit (Collision|LineTraceByChannel _returnvalue_2 (+ (* (Transformation|GetActorForwardVector _returnvalue) 1e+06) _returnvalue_2) "TraceTypeQuery1" false _outactors "None"))
  (if (.bblockinghit _outhit)
    (Transformation|SetWorldRotation _ebbarrel (Math|Conversions|RotationFromXVector (.AimDirection (Class|EBBarrel|CalculateAimDirection (Variables|Components|GetEBBarrelCalc) "/Game/GameFiles/Blueprints/Weapons/NoFallBullets/NoFall_Bullet.NoFall_Bullet_C" (.location _outhit) "0, 0, 0" 1e+01 0.1 4))) false false)
    (else
      (Transformation|SetRelativeRotation _ebbarrel "0.000000,90.000000,0.000000" false false))))

(event Custom|ReloadEvent
  (bind _ebbarrel (Variables|Components|GetEBBarrel))
  ;[0 0.016 1] Reload
  (Components|Animation|PlayAnimation (Variables|Components|GetWeaponMesh) (Variables|WeaponCaracteristics|GetReloadAnimation self) false)
  (Class|EBBarrel|SetAmmo _ebbarrel (Variables|Default|GetAmmoCapacity) false false false (Variables|/Script/EasyBallistics.EBBarrel|GetAmmo _ebbarrel)))

(event Custom|Weapon/BarrelSpreadAndRecoil
  (bind _playerref (Variables|Reference|GetPlayerRef))
  (bind _spreadincreasepershot (Variables|Spread|GetSpreadIncreasePerShot))
  (bind _spreadincreasepershot_2 (Variables|Spread|GetSpreadIncreasePerShot))
  (bind _playerref_2 (Variables|Reference|GetPlayerRef))
  (bind _ebbarrel (Variables|Components|GetEBBarrel))
  (bind _returnvalue (* _spreadincreasepershot 25.0))
  (bind _returnvalue_2 (* _spreadincreasepershot_2 75.0))
  (bind _crosshairhud_ref (Variables|/Game/AdvancedLocomotionV4/Blueprints/CharacterLogic/PlayerCharacter.PlayerCharacter_C|GetCrossHairHud_Ref _playerref_2))
  (bind _returnvalue_3 (/ _returnvalue 2.0))
  (bind _returnvalue_4 (* _returnvalue_2 -1.0))
  (bind _wbcrosshair (Variables|/Game/GameFiles/Blueprints/UI/UI_CrossHair.UI_CrossHair_C|GetWBCrosshair _crosshairhud_ref))
  ;[1 0 0] Weapon: Barre and Crosshair Spread and Recull
  (Utilities|FlowControl|Sequence
    (:then_0
      ;;[1 1 1] EBBarel/Weapon Spread
      (if (< (+ (Variables|/Script/EasyBallistics.EBBarrel|GetSpread _ebbarrel) (Variables|Spread|GetSpreadIncreasePerShot)) (Variables|Spread|GetMaxSpread))
        (Variables|/Script/EasyBallistics.EBBarrel|SetSpread _ebbarrel (+ (Variables|/Script/EasyBallistics.EBBarrel|GetSpread _ebbarrel) (Variables|Spread|GetSpreadIncreasePerShot)))))
    (:then_1
      ;;[1 1 1] WBCosshair Spread
      (if (< (* (Variables|Spread|GetMaxSpread) 1.5e+02) (+ (* (Variables|Spread|GetSpreadIncreasePerShot) 1.5e+02) (Variables|/Game/GameFiles/Blueprints/UI/WBCrosshair.WBCrosshair_C|Getcrosshair_spread _wbcrosshair)))
        (Variables|/Game/GameFiles/Blueprints/UI/WBCrosshair.WBCrosshair_C|Setcrosshair_spread _wbcrosshair (+ (* (Variables|Spread|GetSpreadIncreasePerShot) 1.5e+02) (Variables|/Game/GameFiles/Blueprints/UI/WBCrosshair.WBCrosshair_C|Getcrosshair_spread _wbcrosshair)))))
    (:then_2
      ;;[1 1 1] Recoil
      (Pawn|Input|AddControllerPitchInput _playerref (Math|Random|RandomFloatinRange (/ _returnvalue_4 2.0) _returnvalue_4))
      (Pawn|Input|AddControllerYawInput _playerref (Math|Random|RandomFloatinRange (* -1.0 _returnvalue_3) _returnvalue_3)))))

(event EventBeginPlay
  ;[1 1 1] Get Player Reference
  (bind _asplayer_character (Utilities|Casting|CastToPlayerCharacter (Game|GetPlayerCharacter 0)))
  (Variables|Reference|SetPlayerRef _asplayer_character))

(fn ConstructionScript)

(fn GetWeaponReloadAnimation
  (switch Utilities|FlowControl|Switch|SwitchonWeaponNames (Variables|WeaponCaracteristics|GetWeaponName)
    (:NewEnumerator0
      (return 0))
    (:NewEnumerator1
      (return (Variables|WeaponCaracteristics|GetReloadAnimation)))))