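; Base bullet Blueprint that defines what happens when a shot hits a surface or actor.
; Its OnImpact event branches on the Ricochet flag, with both paths spawning an oriented, timed decal, a splash emitter and a hit sound.
; Only non-ricochet hits apply fixed damage to the hit actor, and ricochets use their own decal material.
; The graph contains no movement or hit detection logic, and the impact impulse does not affect the result.
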(event EventOnImpact
  (params (Ricochet :type Boolean) (PassedThrough :type Boolean) (Location :type Vector :default "0, 0, 0") (IncomingVelocity :type Vector :default "0, 0, 0") (Normal :type Vector :default "0, 0, 0") (ExitLocation :type Vector :default "0, 0, 0") (ExitVelocity :type Vector :default "0, 0, 0") (Impulse :type Vector :default "0, 0, 0") (PenetrationDepth :type Float%20%28single-precision%29) (Actor :type Actor%20Object%20Reference) (Component :type Scene%20Component%20Object%20Reference) (BoneName :type Name :default "None") (PhysMaterial :type Physical%20Material%20Object%20Reference) (HitResult :type Hit%20Result%20Structure))
  (bind _returnvalue (Math|Conversions|RotationFromXVector Normal))
  (bind _returnvalue_2 (Math|Conversions|RotationFromXVector Normal))
  (if Ricochet
    ;[1 1 1] Ricochet
    (Rendering|Decal|SpawnDecalatLocation "/Game/GameFiles/Blueprints/Weapons/Decals/Ricochet_Mat.Ricochet_Mat" "10.000000,10.000000,10.000000" Location _returnvalue 3e+01)
    (Effects|SpawnEmitteratLocation (Variables|Default|GetSplashEffect self) Location _returnvalue)
    (Audio|PlaySoundatLocation (Variables|Default|GetHitSound self) Location "0, 0, 0" 1.0 1.0 0.0 0 0 0 0)
    (else
      ;[1 1 1] Hit on Ground
      (Game|Damage|ApplyDamage Actor 1e+01 0 0 "/Script/Engine.DamageType")
      (Rendering|Decal|SpawnDecalatLocation (Variables|Default|GetDecalMaterial self) "10.000000,10.000000,10.000000" Location _returnvalue_2 3e+01)
      (Effects|SpawnEmitteratLocation (Variables|Default|GetSplashEffect self) Location _returnvalue_2)
      (Audio|PlaySoundatLocation (Variables|Default|GetHitSound self) Location "0, 0, 0" 1.0 1.0 0.0 0 0 0 0))))

(fn ConstructionScript)